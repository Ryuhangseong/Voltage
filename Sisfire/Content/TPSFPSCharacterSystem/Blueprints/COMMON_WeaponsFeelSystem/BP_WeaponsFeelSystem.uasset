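; Weapon feel system that sways the first-person weapon by offsetting arrow components on the player character from look and movement input.
; Each tick it maps controller axes to impact ranges in data tables, scaled by aim or main coefficients from a weapon feel row.
; Range changes start looping timers that ease each delta along fast look or slow move curves.
; A hardcoded branch applies offsets only to the aim arrow, resetting the main arrow.
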(event `InitializeFeelArrows`
  (params (MainArrow :type "ArrowComponent Object Reference") (AimArrow :type "ArrowComponent Object Reference"))
  (set `self.MainArrow` MainArrow)
  (set `self.AimArrow` AimArrow))

(event `InitializeWeaponFeelSettings`
  (params (`Weapon Feel Library Tag` :type Name))
  ;[1 1 1] InitializeWeaponFeelSettings
  (bind _returnvalue (`|GetDataTableRow` (`self.WEAPON FEEL LIBRARY`) `Weapon Feel Library Tag`)
    (:`then`
      (bind (_turnmaincoeffimpact _turnaimcoeffimpact _lockupmaincoeffimpact _lockupaimcoeffimpact _moverightmaincoeffimpact _moverightaimcoeffimpact _moveforwardmaincoeffimpact _moveforwardaimcoeffimpact) (break `/Game/TPSFPSCharacterSystem/Blueprints/COMMON_WeaponsFeelSystem/STR_WeaponFeelSettingDesc` _returnvalue))
      (set `self.Main Coeff Turn Impact` _turnmaincoeffimpact)
      (set `self.Aim Coeff Turn Impact` _turnaimcoeffimpact)
      (set `self.Main Coeff LockUp Impact` _lockupmaincoeffimpact)
      (set `self.Aim Coeff LockUp Impact` _lockupaimcoeffimpact)
      (set `self.Main Coeff Move Right Impact` _moverightmaincoeffimpact)
      (set `self.Aim Coeff Move Right Impact` _moverightaimcoeffimpact)
      (set `self.Main Coeff Move Forward Impact` _moveforwardmaincoeffimpact)
      (set `self.Aim Coeff Move Forward Impact` _moveforwardaimcoeffimpact))))

(event `self.ReceiveBeginPlay`
  ;[1 1 1] EVENT BEGIN PLAY. INITIALIZE THE SYSTEM
  (`KismetSystemLibrary.Delay` 0.2) ; Delay for wait of create charecter with weapon
  (`self.InitializeWeaponFeelSettings` "default")
  (`self.CalculationDefaultArrowsLocRot`)
  (`KismetSystemLibrary.Delay` 0.5) ; Delay for initialize values
  (`self.StartWeaponFeelSystem`) ; Turn On of Event Tick Gate
)

(event `self.ReceiveTick`
  (params (DeltaSeconds :type "Float (single-precision)"))
  ;[1 1 1] EVENT TICK. UPDATE CONROLLER VALUES, IMPACT, RELETIV LOC AND ROT
  (`/Engine/EditorBlueprintResources/StandardMacros.Gate` true :!label _label
    (:`Exit`
      (`self.UpdateControllerValues`) ; Update Axis Values
      (`self.UpdateImpact` :!pinned true) ; UPDATE IMPACT
      (`self.CalculationCurrentArrowsLocRot`)
      (`self.UpdateMechLocRot`))))

(event `MiniZoomOn`
  ;[1 0.4103 0.7607] Update Minizoom state
  (set `self.In Minizoom?` true))

(event `MiniZoomOff`
  ;[1 0.4103 0.7607] Update Minizoom state
  (set `self.In Minizoom?` false))

(event `StartWeaponFeelSystem`
  ;[1 1 1] EVENT TICK. UPDATE CONROLLER VALUES, IMPACT, RELETIV LOC AND ROT
  (goto _label :!via `Open`))

(event `TurnStartInterpolation`
  ;[1 1 1] START TURN INTERPOLATION
  ;;[1 1 1] Start / Stop
  (`self.TurnInterpolationStep`)
  (`KismetSystemLibrary.K2_SetTimer` null "TurnInterpolationStep" (`self.IntStep`) true))

(event `TurnInterpolationStep`
  ;[1 1 1] START TURN INTERPOLATION
  ;;[1 1 1] Step
  (if (== (`self.TurnNewDelta`) (`self.TurnCurrentDelta`))
    (`self.TurnStopInterpolation`)
    (else
      (bind _output_get (set `self.TurnCurveTime` (+ (`self.TurnCurveTime`) (`self.IntStep`))))
      (set `self.TurnCurrentDelta` (`|EaseFunction` "Linear" (`CurveFloat.GetFloatValue` (`self.WeaponFeelTransitionCurveFast`) _output_get) (`self.TurnOldDelta`) (`self.TurnNewDelta`))))))

(event `TurnOpenGate`
  ;[1 1 1] UPDATE IMPACT
  ;;[1 1 1] TURN IMPACT
  ;;;[1 1 1] Range Changed Condition
  (goto _label_2 :!via `Reset`))

(event `TurnStopInterpolation`
  ;[1 1 1] START TURN INTERPOLATION
  ;;[1 1 1] Start / Stop
  (`KismetSystemLibrary.K2_ClearTimer` null "TurnInterpolationStep")
  (set `self.TurnCurveTime` 0.0))

(event `UpdateImpact`
  ;[1 1 1] UPDATE IMPACT
  (`|ExecutionSequence`
    (:`then_0`
      ;;[1 1 1] TURN IMPACT
      ;;;[1 1 1] Range and Impact Value Definition
      (bind (_impact_value _impact_range) (`self.RangeDefinition` "/Game/TPSFPSCharacterSystem/Blueprints/COMMON_WeaponsFeelSystem/ComponentValues/DT_WeaponFeelTurnRanges.DT_WeaponFeelTurnRanges" (`self.Input Turn Axis Value`) (`self.Aim Coeff Turn Impact`) (`self.Main Coeff Turn Impact`)))
      (set `self.TurnImpactValue` _impact_value)
      (set `self.TurnNewRange` _impact_range)
      ;;;[1 1 1] Range Changed Condition
      (if (not (== (`self.TurnNewRange`) (`self.TurnCurrentRange`)))
        (`/Engine/EditorBlueprintResources/StandardMacros.DoOnce` false :!label _label_2
          (:`Completed`
            (set `self.TurnCurrentRange` (`self.TurnNewRange`))
            ;;;[1 1 1] START TURN INTERPOLATION
            (`self.TurnStopInterpolation`)
            (set `self.TurnOldDelta` (`self.TurnCurrentDelta`))
            (set `self.TurnNewDelta` (`self.TurnImpactValue`))
            (`self.TurnStartInterpolation`)
            (`self.TurnOpenGate`)))))
    (:`then_1`
      ;;[1 1 1] LOCK UP IMPACT
      ;;;[1 1 1] Range and Impact Value Definition
      (bind (_impact_value_2 _impact_range_2) (`self.RangeDefinition` "/Game/TPSFPSCharacterSystem/Blueprints/COMMON_WeaponsFeelSystem/ComponentValues/DT_WeaponFeelLockUpRanges.DT_WeaponFeelLockUpRanges" (`self.Input LockUp Axis Value`) (`self.Aim Coeff LockUp Impact`) (`self.Main Coeff LockUp Impact`)))
      (set `self.LockUpImpactValue` _impact_value_2)
      (set `self.LookUpNewRange` _impact_range_2)
      ;;;[1 1 1] Range Changed Condition
      (if (not (== (`self.LookUpNewRange`) (`self.LockUpCurrentRange`)))
        (`/Engine/EditorBlueprintResources/StandardMacros.DoOnce` false :!label _label_3
          (:`Completed`
            (set `self.LockUpCurrentRange` (`self.LookUpNewRange`))
            ;;;[1 1 1] START LOCK UP INTERPOLATION
            (`self.LockUpStopInterpolation`)
            (set `self.LockUpOldDelta` (`self.LockUpCurrentDelta`))
            (set `self.LockUpNewDelta` (`self.LockUpImpactValue`))
            (`self.LockUpStartInterpolation`)
            (`self.LockUpOpenGate`)))))
    (:`then_2`
      ;;[1 0.4103 0.7607] Off if minizoom with CoD Style
      (if (and (`self.MainStyleAim?`) (`self.In Minizoom?`))
        (set `self.Out Move Right Axis Value` 0.0)
        (else
          (set `self.Out Move Right Axis Value` (`self.Input Move Right Axis Value`))))
      ;;[1 1 1] MOVE RIGHT IMPACT
      ;;;[1 1 1] Range and Impact Value Definition
      (bind (_impact_value_3 _impact_range_3) (`self.RangeDefinition` "/Game/TPSFPSCharacterSystem/Blueprints/COMMON_WeaponsFeelSystem/ComponentValues/DT_WeaponFeelMoveRightRanges.DT_WeaponFeelMoveRightRanges" (`self.Out Move Right Axis Value`) (`self.Aim Coeff Move Right Impact`) (`self.Main Coeff Move Right Impact`)))
      (set `self.MoveRightImpactValue` _impact_value_3)
      (set `self.MoveRightNewRange` _impact_range_3)
      ;;;[1 1 1] Range Changed Condition
      (if (not (== (`self.MoveRightNewRange`) (`self.MoveRightCurrentRange`)))
        (`/Engine/EditorBlueprintResources/StandardMacros.DoOnce` false :!label _label_4
          (:`Completed`
            (set `self.MoveRightCurrentRange` (`self.MoveRightNewRange`))
            ;;;[1 1 1] START MOVE RIGHT INTERPOLATION
            (`self.MoveRightStopInterpolation`)
            (set `self.MoveRightOldDelta` (`self.MoveRightCurrentDelta`))
            (set `self.MoveRightNewDelta` (`self.MoveRightImpactValue`))
            (`self.MoveRightStartInterpolation`)
            (`self.MoveRightOpenGate`)))))
    (:`then_3`
      (if (and (`self.MainStyleAim?`) (`self.In Minizoom?`))
        (set `self.Out Move Forward Axis Value` 0.0)
        (else
          (set `self.Out Move Forward Axis Value` (`self.Input Move Forward Axis Value`))))
      ;;[1 1 1] MOVE FORWARD IMPACT
      ;;;[1 1 1] Range and Impact Value Definition
      (bind (_impact_value_4 _impact_range_4) (`self.RangeDefinition` "/Game/TPSFPSCharacterSystem/Blueprints/COMMON_WeaponsFeelSystem/ComponentValues/DT_WeaponFeelMoveForwardRanges.DT_WeaponFeelMoveForwardRanges" (`self.Out Move Forward Axis Value`) (`self.Aim Coeff Move Forward Impact`) (`self.Main Coeff Move Forward Impact`)))
      (set `self.MoveForwardImpactValue` _impact_value_4)
      (set `self.MoveForwardNewRange` _impact_range_4)
      ;;;[1 1 1] Range Changed Condition
      (if (not (== (`self.MoveForwardNewRange`) (`self.MoveForwardCurrentRange`)))
        (`/Engine/EditorBlueprintResources/StandardMacros.DoOnce` false :!label _label_5
          (:`Completed`
            (set `self.MoveForwardCurrentRange` (`self.MoveForwardNewRange`))
            ;;;[1 1 1] START MOVE FORWARD INTERPOLATION
            (`self.MoveForwardStopInterpolation`)
            (set `self.MoveForwardOldDelta` (`self.MoveForwardCurrentDelta`))
            (set `self.MoveForwardNewDelta` (`self.MoveForwardImpactValue`))
            (`self.MoveForwardStartInterpolation`)
            (`self.MoveForwardOpenGate`)))))))

(event `LockUpOpenGate`
  ;[1 1 1] UPDATE IMPACT
  ;;[1 1 1] LOCK UP IMPACT
  ;;;[1 1 1] Range Changed Condition
  (goto _label_3 :!via `Reset`))

(event `LockUpStartInterpolation`
  ;[1 1 1] START LOCK UP INTERPOLATION
  ;;[1 1 1] Start / Stop
  (`self.LockUpInterpolationStep`)
  (`KismetSystemLibrary.K2_SetTimer` null "LockUpInterpolationStep" (`self.IntStep`) true))

(event `LockUpInterpolationStep`
  ;[1 1 1] START LOCK UP INTERPOLATION
  ;;[1 1 1] Step
  (if (== (`self.LockUpNewDelta`) (`self.LockUpCurrentDelta`))
    (`self.LockUpStopInterpolation`)
    (else
      (bind _output_get (set `self.LockUpCurveTime` (+ (`self.LockUpCurveTime`) (`self.IntStep`))))
      (set `self.LockUpCurrentDelta` (`|EaseFunction` "Linear" (`CurveFloat.GetFloatValue` (`self.WeaponFeelTransitionCurveFast`) _output_get) (`self.LockUpOldDelta`) (`self.LockUpNewDelta`))))))

(event `LockUpStopInterpolation`
  ;[1 1 1] START LOCK UP INTERPOLATION
  ;;[1 1 1] Start / Stop
  (`KismetSystemLibrary.K2_ClearTimer` null "LockUpInterpolationStep")
  (set `self.LockUpCurveTime` 0.0))

(event `MoveRightOpenGate`
  ;[1 1 1] UPDATE IMPACT
  ;;[1 1 1] MOVE RIGHT IMPACT
  ;;;[1 1 1] Range Changed Condition
  (goto _label_4 :!via `Reset`))

(event `MoveRightStartInterpolation`
  ;[1 1 1] START MOVE RIGHT INTERPOLATION
  ;;[1 1 1] Start / Stop
  (`self.MoveRightInterpolationStep`)
  (`KismetSystemLibrary.K2_SetTimer` null "MoveRightInterpolationStep" (`self.IntStep`) true))

(event `MoveRightInterpolationStep`
  ;[1 1 1] START MOVE RIGHT INTERPOLATION
  ;;[1 1 1] Step
  (if (== (`self.MoveRightNewDelta`) (`self.MoveRightCurrentDelta`))
    (`self.MoveRightStopInterpolation`)
    (else
      (bind _output_get (set `self.MoveRightCurveTime` (+ (`self.MoveRightCurveTime`) (`self.IntStep`))))
      (set `self.MoveRightCurrentDelta` (`|EaseFunction` "Linear" (`CurveFloat.GetFloatValue` (`self.WeaponFeelTransitionCurveSlow`) _output_get) (`self.MoveRightOldDelta`) (`self.MoveRightNewDelta`))))))

(event `MoveForwardOpenGate`
  ;[1 1 1] UPDATE IMPACT
  ;;[1 1 1] MOVE FORWARD IMPACT
  ;;;[1 1 1] Range Changed Condition
  (goto _label_5 :!via `Reset`))

(event `MoveRightStopInterpolation`
  ;[1 1 1] START MOVE RIGHT INTERPOLATION
  ;;[1 1 1] Start / Stop
  (`KismetSystemLibrary.K2_ClearTimer` null "MoveRightInterpolationStep")
  (set `self.MoveRightCurveTime` 0.0))

(event `MoveForwardStartInterpolation`
  ;[1 1 1] START MOVE FORWARD INTERPOLATION
  ;;[1 1 1] Start / Stop
  (`self.MoveForwardInterpolationStep`)
  (`KismetSystemLibrary.K2_SetTimer` null "MoveForwardInterpolationStep" (`self.IntStep`) true))

(event `MoveForwardInterpolationStep`
  ;[1 1 1] START MOVE FORWARD INTERPOLATION
  ;;[1 1 1] Step
  (if (== (`self.MoveForwardNewDelta`) (`self.MoveForwardCurrentDelta`))
    (`self.MoveForwardStopInterpolation`)
    (else
      (bind _output_get (set `self.MoveForwardCurveTime` (+ (`self.MoveForwardCurveTime`) (`self.IntStep`))))
      (set `self.MoveForwardCurrentDelta` (`|EaseFunction` "Linear" (`CurveFloat.GetFloatValue` (`self.WeaponFeelTransitionCurveSlow`) _output_get) (`self.MoveForwardOldDelta`) (`self.MoveForwardNewDelta`))))))

(event `MoveForwardStopInterpolation`
  ;[1 1 1] START MOVE FORWARD INTERPOLATION
  ;;[1 1 1] Start / Stop
  (`KismetSystemLibrary.K2_ClearTimer` null "MoveForwardInterpolationStep")
  (set `self.MoveForwardCurveTime` 0.0))

(fn `CalculationCurrentArrowsLocRot`
  (bind _impactcoeffminizoom (`self.ImpactCoeffMinizoom`))
  ;[1 1 1] CurrentFloorArrowRotation
  (bind _output_get (set `self.CurrentFloorArrowRotation` (`KismetMathLibrary.MakeRotator` (`self.MoveRightCurrentDelta`) (`self.LockUpCurrentDelta`) (`self.TurnCurrentDelta`))))
  ;[1 1 1] CurrentMiniZoomArrowRotation
  (set `self.CurrentMiniZoomArrowRotation` (`KismetMathLibrary.MakeRotator` (* (.roll _output_get) _impactcoeffminizoom) (* (.pitch _output_get) _impactcoeffminizoom) (* (.yaw _output_get) _impactcoeffminizoom)))
  ;[1 1 1] CurrentFloorArrowLocation
  (set `self.CurrentFloorArrowLocation` (`KismetMathLibrary.MakeVector` (+ (`self.MoveForwardCurrentDelta`) (.x (`self.DefaultFloorArrowLocation`))) (+ (.y (`self.DefaultFloorArrowLocation`)) (`self.MoveRightCurrentDelta`)) (.z (`self.DefaultFloorArrowLocation`))))
  ;[1 1 1] CurrentMiniZoomArrowLocation
  (set `self.CurrentMiniZoomArrowLocation` (`KismetMathLibrary.MakeVector` (+ (* (`self.MoveForwardCurrentDelta`) (`self.ImpactCoeffMinizoom`)) (.x (`self.DefaultMiniZoomArrowLocation`))) (+ (.y (`self.DefaultMiniZoomArrowLocation`)) (* (`self.MoveRightCurrentDelta`) (`self.ImpactCoeffMinizoom`))) (.z (`self.DefaultMiniZoomArrowLocation`)))))

(fn `CalculationDefaultArrowsLocRot`
  (bind _asbp_basic_fpscharacter (cast `/Game/TPSFPSCharacterSystem/Blueprints/BASIC_FPSCharacter/BP_BASIC_FPSCharacter` (`GameplayStatics.GetPlayerPawn` 0)))
  (bind _weaponfeelarrowmain (`/Game/TPSFPSCharacterSystem/Blueprints/BASIC_FPSCharacter/BP_BASIC_FPSCharacter.WeaponFeelArrowMain` _asbp_basic_fpscharacter))
  (set `self.DefaultRotation` (`SceneComponent.RelativeRotation` _weaponfeelarrowmain))
  (set `self.DefaultFloorArrowLocation` (`SceneComponent.RelativeLocation` _weaponfeelarrowmain))
  (bind _weaponfeelarrowaim (`/Game/TPSFPSCharacterSystem/Blueprints/BASIC_FPSCharacter/BP_BASIC_FPSCharacter.WeaponFeelArrowAim` _asbp_basic_fpscharacter))
  (set `self.DefaultMiniZoomArrowLocation` (`SceneComponent.RelativeLocation` _weaponfeelarrowaim))
  (`self.InitializeFeelArrows` _weaponfeelarrowmain _weaponfeelarrowaim))

(fn `CheckingImpactValueDirection`
  (params (`Impact Value` :type "Float (double-precision)"))
  (returns (`Was Changed Direction?` :type Boolean))
  (locals (NewImpactValue :type "Float (double-precision)") (OldImpactValue :type "Float (double-precision)") (`NewValueHaveNewDirection?` :type Boolean))
  (set `local.NewImpactValue` `Impact Value`)
  (if (> (`local.NewImpactValue`) 0.0)
    (if (and (> (`local.NewImpactValue`) 0.0) (> (`local.OldImpactValue`) 0.0))
      (set `local.NewValueHaveNewDirection?` false)
      (else
        (set `local.NewValueHaveNewDirection?` true)))
    (elif (and (< (`local.NewImpactValue`) 0.0) (< (`local.OldImpactValue`) 0.0))
      (set `local.NewValueHaveNewDirection?` false)
      (else
        (set `local.NewValueHaveNewDirection?` true))))
  (set `local.OldImpactValue` (`local.NewImpactValue`))
  (return (`local.NewValueHaveNewDirection?`)))

(fn `RangeDefinition`
  (params (`Data Table` :type "DataTable Object Reference") (`Axis Value` :type "Float (double-precision)") (`MiniZoom Coeff` :type "Float (double-precision)") (`Floor Coeff` :type "Float (double-precision)"))
  (returns (`Impact Value` :type "Float (double-precision)") (`Impact Range` :type Name))
  (locals (ImpactValue :type "Float (double-precision)") (ImpactRange :type Name) (AxixValue :type "Float (double-precision)") (MiniZoomCoeff :type "Float (double-precision)") (FloorCoeff :type "Float (double-precision)"))
  (set `local.AxixValue` `Axis Value`)
  (set `local.MiniZoomCoeff` `MiniZoom Coeff`)
  (set `local.FloorCoeff` `Floor Coeff`)
  (bind _outrownames (`DataTableFunctionLibrary.GetDataTableRowNames` `Data Table`))
  (for _array_element _outrownames
    (bind _returnvalue (`|GetDataTableRow` `Data Table` _array_element)
      (:`then`
        (bind (_minaxisvalue _maxaxisvalue _impactvalue) (break `/Game/TPSFPSCharacterSystem/Blueprints/COMMON_WeaponsFeelSystem/ComponentValues/STR_WeaponFeelRangeDescribe` _returnvalue))
        (if (`KismetMathLibrary.InRange_FloatFloat` (`local.AxixValue`) _minaxisvalue _maxaxisvalue)
          (set `local.ImpactRange` _array_element)
          ;[1 0.4103 0.7607] Mini Zoom Coeff
          (if (and (`self.MainStyleAim?`) (`self.In Minizoom?`))
            (set `local.ImpactValue` (* _impactvalue (`local.MiniZoomCoeff`)))
            (else
              (set `local.ImpactValue` (* _impactvalue (`local.FloorCoeff`)))))
          (return (`local.ImpactValue`) (`local.ImpactRange`)))))))

(fn `TransitionSpeedDefinition`
  (params (`Current Range` :type Name) (`New Range` :type Name))
  (returns (`Speed Coeff` :type "Float (double-precision)"))
  (locals (LocCurrentRange :type Integer) (LocNewRange :type Integer) (DeltaRange :type Integer) (SpeedCoeff :type "Float (double-precision)"))
  (set `local.LocCurrentRange` (`KismetStringLibrary.Conv_StringToInt` (`KismetStringLibrary.Conv_NameToString` `Current Range`)))
  (set `local.LocNewRange` (`KismetStringLibrary.Conv_StringToInt` (`KismetStringLibrary.Conv_NameToString` `New Range`)))
  (bind _output_get (set `local.DeltaRange` (`KismetMathLibrary.Abs_Int` (- (`local.LocCurrentRange`) (`local.LocNewRange`)))))
  (switch `int` _output_get
    (:`0`
      (set `local.SpeedCoeff` 1.0))
    (:`1`
      (set `local.SpeedCoeff` 0.8))
    (:`2`
      (set `local.SpeedCoeff` 0.7))
    (:`3`
      (set `local.SpeedCoeff` 0.6))
    (:`4`
      (set `local.SpeedCoeff` 0.5)))
  (return (`local.SpeedCoeff`)))

(fn `UpdateControllerValues`
  (locals (`UseMouse?` :type Boolean :default false))
  (bind _asbp_common_player_controller (cast `/Game/TPSFPSCharacterSystem/Blueprints/COMMON_PlayerController/BP_CommonPlayerController` (`GameplayStatics.GetPlayerController` 0)))
  (set `local.UseMouse?` (`/Game/TPSFPSCharacterSystem/Blueprints/COMMON_PlayerController/BP_CommonPlayerController.UseMouse?` _asbp_common_player_controller))
  ;[1 1 1] Set Controller Values
  (set `self.Input Move Forward Axis Value` (`/Game/TPSFPSCharacterSystem/Blueprints/COMMON_PlayerController/BP_CommonPlayerController.Pre Move Forward Axis Value` _asbp_common_player_controller))
  (set `self.Input Move Right Axis Value` (`/Game/TPSFPSCharacterSystem/Blueprints/COMMON_PlayerController/BP_CommonPlayerController.Pre Move Right Axis Value` _asbp_common_player_controller))
  (if (`local.UseMouse?`)
    (set `self.Input Turn Axis Value` (`/Game/TPSFPSCharacterSystem/Blueprints/COMMON_PlayerController/BP_CommonPlayerController.Initial Turn Mouse Input Axis Value` _asbp_common_player_controller))
    (set `self.Input LockUp Axis Value` (`/Game/TPSFPSCharacterSystem/Blueprints/COMMON_PlayerController/BP_CommonPlayerController.Initial LockUp Mouse Input Axis Value` _asbp_common_player_controller))
    (else
      (set `self.Input Turn Axis Value` (`/Game/TPSFPSCharacterSystem/Blueprints/COMMON_PlayerController/BP_CommonPlayerController.Final Turn Axis Value` _asbp_common_player_controller))
      (set `self.Input LockUp Axis Value` (`/Game/TPSFPSCharacterSystem/Blueprints/COMMON_PlayerController/BP_CommonPlayerController.Final LockUp Axis Value` _asbp_common_player_controller)))))

(fn `UpdateFeelCoefficients`)

(fn `UpdateMechLocRot`
  (bind _asbp_basic_fpscharacter (cast `/Game/TPSFPSCharacterSystem/Blueprints/BASIC_FPSCharacter/BP_BASIC_FPSCharacter` (`GameplayStatics.GetPlayerPawn` 0)))
  (set `self.In Minizoom?` (`/Game/TPSFPSCharacterSystem/Blueprints/COMMON_CommonCharacter/BP_CommonCharacter.GetAimStates` _asbp_basic_fpscharacter))
  (if true
    (`|ExecutionSequence`
      (:`then_0`
        (bind _weaponfeelarrowaim (`/Game/TPSFPSCharacterSystem/Blueprints/BASIC_FPSCharacter/BP_BASIC_FPSCharacter.WeaponFeelArrowAim` _asbp_basic_fpscharacter))
        (`SceneComponent.K2_SetRelativeLocationAndRotation` _weaponfeelarrowaim (`self.CurrentMiniZoomArrowLocation`) (`self.CurrentMiniZoomArrowRotation`) true false))
      (:`then_1`
        (bind _weaponfeelarrowmain (`/Game/TPSFPSCharacterSystem/Blueprints/BASIC_FPSCharacter/BP_BASIC_FPSCharacter.WeaponFeelArrowMain` _asbp_basic_fpscharacter))
        (`SceneComponent.K2_SetRelativeLocationAndRotation` _weaponfeelarrowmain (`self.DefaultFloorArrowLocation`) (`self.DefaultRotation`) true false)))
    (else
      (`|ExecutionSequence`
        (:`then_0`
          (`SceneComponent.K2_SetRelativeLocationAndRotation` _weaponfeelarrowmain (`self.CurrentFloorArrowLocation`) (`self.CurrentFloorArrowRotation`) true false))
        (:`then_1`
          (`SceneComponent.K2_SetRelativeLocationAndRotation` _weaponfeelarrowaim (`self.DefaultMiniZoomArrowLocation`) (`self.DefaultRotation`) true false))))))
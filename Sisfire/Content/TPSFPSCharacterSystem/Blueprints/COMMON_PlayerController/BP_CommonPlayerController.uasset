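; Player controller for the TPS/FPS character system that creates the main HUD, forwards input actions to the controlled common character and requests respawns from the game mode.
; Actions call the character or its weapon system for shooting, aim, melee, cover, camera and stance, with timed crouch holds toggling prone.
; Axis handlers apply interpolated, yaw-relative movement, constrained during sprint, plus mouse and gamepad look.
; A V key shortcut refills health.
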(event `CreateCommonPlayerHUD`
  ;[1 1 1] CreateCommonPlayerHUD
  (`/Engine/EditorBlueprintResources/StandardMacros.DoOnce` false
    (:`Completed`
      (bind _returnvalue (`|CreateWidget` "/Game/TPSFPSCharacterSystem/Blueprints/COMMON_HUD/WBP_CommonMainHUD.WBP_CommonMainHUD_C"))
      (bind _output_get (set `self.HUD` _returnvalue))
      (`/Engine/EditorBlueprintResources/StandardMacros.IsValid` _output_get
        (:`Is Valid`
          (`UserWidget.AddToPlayerScreen` _output_get 3))))))

(event `Key|V`
  (params (Key :type "Key Structure"))
  ;[1 1 1] Heal Player
  (:`Pressed`
    (bind _asbp_basic_tpsfpscharacter (cast `/Game/TPSFPSCharacterSystem/Blueprints/BASIC_TPSFPSCharacter/BP_BASIC_TPSFPSCharacter` (`GameplayStatics.GetPlayerCharacter` 0)))
    (bind _output_get (set `/Game/TPSFPSCharacterSystem/Blueprints/BASIC_TPSFPSCharacter/BP_BASIC_TPSFPSCharacter.HealthForLifeBar` 10000.0 _asbp_basic_tpsfpscharacter))
    (bind _asbp_basic_base_character (cast `/Game/TPSFPSCharacterSystem/Blueprints/BASIC_BaseCharacter/BP_BASIC_BaseCharacter` (`GameplayStatics.GetPlayerCharacter` 0)))
    (`/Game/TPSFPSCharacterSystem/Blueprints/COMMON_CommonCharacter/BP_CommonCharacter.UpdateCurrentHealth` _asbp_basic_base_character _output_get)))

(event `self.ReceiveBeginPlay`
  ;[1 1 1] EVENT BEGIN PLAY
  (`|ExecutionSequence`
    (:`then_0`
      (`self.CreateCommonPlayerHUD`))
    (:`then_1`
      (`self.DisableInput` null)
      (`KismetSystemLibrary.Delay` 0.2)
      (`self.EnableInput` null))))

(event `self.ReceiveTick`
  (params (DeltaSeconds :type "Float (single-precision)"))
  (bind _returnvalue (`KismetMathLibrary.MakeRotator` 0.0 0.0 (.yaw (`Pawn.GetControlRotation` (`self.K2_GetPawn`)))))
  ;[1 1 1] EVENT TICK
  (set `self.DeltaSeconds` DeltaSeconds)
  ;;[1 1 1] Calculation Forward and Right Vectors
  (`/Engine/EditorBlueprintResources/StandardMacros.IsValid` (`self.K2_GetPawn`)
    (:`Is Valid`
      (set `self.Forward Vector` (`KismetMathLibrary.GetForwardVector` _returnvalue))
      (set `self.Right Vector` (`KismetMathLibrary.GetRightVector` _returnvalue)))))

(event `InputAction|ReloadPC`
  (params (Key :type "Key Structure"))
  ;[1 1 1] Reload / Interaction
  (:`Pressed`
    (`/Game/TPSFPSCharacterSystem/Blueprints/COMMON_CommonCharacter/BP_CommonCharacter.ServerReloadTrigger` (`self.GetCommonCharacter`))))

(event `InputAction|Melee`
  (params (Key :type "Key Structure"))
  ;[1 1 1] MELEE
  (:`Pressed`
    (`/Engine/EditorBlueprintResources/StandardMacros.IsValid` (`self.GetCommonCharacter`)
      (:`Is Valid`
        (`/Game/TPSFPSCharacterSystem/Blueprints/COMMON_CommonCharacter/BP_CommonCharacter.ServerMelee` (`self.GetCommonCharacter`))))))

(event `InputAction|CameraMirrorKeyBoard`
  (params (Key :type "Key Structure"))
  ;[1 1 1] CameraMirror / Scope ZoomOn GamePad
  (:`Pressed`
    (`/Game/TPSFPSCharacterSystem/Blueprints/COMMON_CommonCharacter/BP_CommonCharacterInterface.CameraMirrow` (`self.GetCommonCharacter`))))

(event `InputAction|Jump`
  (params (Key :type "Key Structure"))
  ;[1 1 1] COVER / JUMP
  (:`Pressed`
    (`/Game/TPSFPSCharacterSystem/Blueprints/COMMON_CommonCharacter/BP_CommonCharacter.CoversInterAction` (`self.GetCommonCharacter`))))

(event `InputAction|ChangeCameraMode`
  (params (Key :type "Key Structure"))
  ;[1 1 1] TPS - FPS
  (:`Pressed`
    (`/Game/TPSFPSCharacterSystem/Blueprints/COMMON_CommonCharacter/BP_CommonCharacterInterface.SwitchTPSFPSCameraMode` (`self.GetCommonCharacter`))))

(event `InputAction|Interaction`
  (params (Key :type "Key Structure"))
  ;[1 1 1] Reload / Interaction
  (:`Pressed`
    (if (`|EnumEquality` (`/Game/TPSFPSCharacterSystem/Blueprints/COMMON_CommonCharacter/BP_CommonCharacter.GetInteractionType` (`self.GetCommonCharacter`)) "NewEnumerator3")
      (`/Game/TPSFPSCharacterSystem/Blueprints/COMMON_CommonCharacter/BP_CommonCharacter.ServerReloadTrigger` (`self.GetCommonCharacter`))
      (else
        (`/Game/TPSFPSCharacterSystem/Blueprints/COMMON_CommonCharacter/BP_CommonCharacter.ClientInteraction` (`self.GetCommonCharacter`))))))

(event `InputAction|CameraMirrorGamePad`
  (params (Key :type "Key Structure"))
  ;[1 1 1] CameraMirror / Scope ZoomOn GamePad
  (:`Pressed`
    (if (`/Game/TPSFPSCharacterSystem/Blueprints/COMMON_WeaponSystem/BP_WeaponSystem.GetHoldAimState` (`/Game/TPSFPSCharacterSystem/Blueprints/COMMON_CommonCharacter/BP_CommonCharacter.BP_WeaponSystem` (`self.GetCommonCharacter`)))
      (if (not (`|EnumEquality` (`/Game/TPSFPSCharacterSystem/Blueprints/COMMON_WeaponSystem/BP_WeaponSystem.GetWeaponScopeType` (`/Game/TPSFPSCharacterSystem/Blueprints/COMMON_CommonCharacter/BP_CommonCharacter.BP_WeaponSystem` (`self.GetCommonCharacter`))) "NewEnumerator0"))
        (`/Game/TPSFPSCharacterSystem/Blueprints/COMMON_WeaponSystem/BP_WeaponSystem.UpdateScopeZoom` (`/Game/TPSFPSCharacterSystem/Blueprints/COMMON_CommonCharacter/BP_CommonCharacter.BP_WeaponSystem` (`self.GetCommonCharacter`)) false false true)
        (else
          (`/Game/TPSFPSCharacterSystem/Blueprints/COMMON_CommonCharacter/BP_CommonCharacterInterface.CameraMirrow` (`self.GetCommonCharacter`))))
      (else
        (`/Game/TPSFPSCharacterSystem/Blueprints/COMMON_CommonCharacter/BP_CommonCharacterInterface.CameraMirrow` (`self.GetCommonCharacter`))))))

(event `InputAction|Interaction`
  (params (Key :type "Key Structure"))
  ;[1 1 1] INTERACTION
  (:`Pressed`
    (`/Game/TPSFPSCharacterSystem/Blueprints/COMMON_CommonCharacter/BP_CommonCharacter.ServerInteraction` (`self.GetCommonCharacter`))))

(event `InputAction|Aim`
  (params (Key :type "Key Structure"))
  ;[1 1 1] AIM
  (:`Pressed`
    (set `self.AimHolding?` true)
    (`/Game/TPSFPSCharacterSystem/Blueprints/COMMON_CommonCharacter/BP_CommonCharacter.ClientAimOn` (`self.GetCommonCharacter`)))
  (:`Released`
    (set `self.AimHolding?` false)
    (`/Game/TPSFPSCharacterSystem/Blueprints/COMMON_CommonCharacter/BP_CommonCharacter.ClientAimOff` (`self.GetCommonCharacter`))))

(event `InputAction|SwapHideWeapon`
  (params (Key :type "Key Structure"))
  ;[1 1 1] SWAP
  (:`Pressed`
    (`/Game/TPSFPSCharacterSystem/Blueprints/COMMON_CommonCharacter/BP_CommonCharacter.ClientSwapWeapon` (`self.GetCommonCharacter`))))

(event `TriggerProneOff`
  ;[1 1 1] CROUCH & PRONE
  (if (`self.CrouchHold?`)
    (if (not (`/Game/TPSFPSCharacterSystem/Blueprints/COMMON_CommonCharacter/BP_CommonCharacter.GetProneState` (`self.GetCommonCharacter`)))
      (`/Game/TPSFPSCharacterSystem/Blueprints/COMMON_CommonCharacter/BP_CommonCharacter.ClientCrouchOff` (`self.GetCommonCharacter`)))))

(event `InputAction|Shot`
  (params (Key :type "Key Structure"))
  ;[1 1 1] SHOOTING
  (:`Pressed`
    (`/Game/TPSFPSCharacterSystem/Blueprints/COMMON_CommonCharacter/BP_CommonCharacter.ServerShootingTriggerOn` (`self.GetCommonCharacter`)))
  (:`Released`
    (`/Game/TPSFPSCharacterSystem/Blueprints/COMMON_CommonCharacter/BP_CommonCharacter.ServerShootingTriggerOff` (`self.GetCommonCharacter`))))

(event `InputAction|ScopeZoomUp`
  (params (Key :type "Key Structure"))
  ;[1 1 1] Score Zoom Up / Down
  (:`Pressed`
    (`/Game/TPSFPSCharacterSystem/Blueprints/COMMON_WeaponSystem/BP_WeaponSystem.UpdateScopeZoom` (`/Game/TPSFPSCharacterSystem/Blueprints/COMMON_CommonCharacter/BP_CommonCharacter.BP_WeaponSystem` (`self.GetCommonCharacter`)) true false false)))

(event `SprintOff`
  ;[1 1 1] SPRINT
  (`/Game/TPSFPSCharacterSystem/Blueprints/COMMON_CommonCharacter/BP_CommonCharacter.ServerSprintOff` (`self.GetCommonCharacter`) :!label _label))

(event `InputAction|Crouch`
  (params (Key :type "Key Structure"))
  ;[1 1 1] CROUCH & PRONE
  (:`Pressed`
    (set `self.CrouchHold?` true)
    (if (`/Game/TPSFPSCharacterSystem/Blueprints/COMMON_CommonCharacter/BP_CommonCharacter.GetProneState` (`self.GetCommonCharacter`))
      (`KismetSystemLibrary.K2_SetTimerDelegate` (delegate `TriggerProneOff`) 0.3)
      (`self.ProneStateInputOff`)
      (else
        (`KismetSystemLibrary.K2_SetTimerDelegate` (delegate `TriggerProneOn`) 0.3)
        (if (`/Game/TPSFPSCharacterSystem/Blueprints/COMMON_CommonCharacter/BP_CommonCharacter.GetCrouchState` (`self.GetCommonCharacter`))
          (`/Game/TPSFPSCharacterSystem/Blueprints/COMMON_CommonCharacter/BP_CommonCharacter.ClientCrouchOff` (`self.GetCommonCharacter`))
          (else
            (`/Game/TPSFPSCharacterSystem/Blueprints/COMMON_CommonCharacter/BP_CommonCharacter.ClientCrouchOn` (`self.GetCommonCharacter`)))))))
  (:`Released`
    (set `self.CrouchHold?` false)))

(event `InputAction|Sprint`
  (params (Key :type "Key Structure"))
  ;[1 1 1] SPRINT
  (:`Pressed`
    (if (`/Game/TPSFPSCharacterSystem/Blueprints/COMMON_CommonCharacter/BP_CommonCharacter.GetSprintState` (`self.GetCommonCharacter`))
      (goto _label)
      (elif (>= (`self.Initial Move Forward Input Axis Value`) 0.5)
        (`/Game/TPSFPSCharacterSystem/Blueprints/COMMON_CommonCharacter/BP_CommonCharacter.ServerSprintOn` (`self.GetCommonCharacter`))))))

(event `InputAction|ScopeZoomDown`
  (params (Key :type "Key Structure"))
  ;[1 1 1] Score Zoom Up / Down
  (:`Pressed`
    (`/Game/TPSFPSCharacterSystem/Blueprints/COMMON_WeaponSystem/BP_WeaponSystem.UpdateScopeZoom` (`/Game/TPSFPSCharacterSystem/Blueprints/COMMON_CommonCharacter/BP_CommonCharacter.BP_WeaponSystem` (`self.GetCommonCharacter`)) false true false)))

(event `TriggerProneOn`
  ;[1 1 1] CROUCH & PRONE
  (if (`self.CrouchHold?`)
    (if (`/Game/TPSFPSCharacterSystem/Blueprints/COMMON_CommonCharacter/BP_CommonCharacter.GetCrouchState` (`self.GetCommonCharacter`))
      (`self.ProneStateInputOn`))))

(event `RespawnPlayerCharacter`
  (params (`Player Controller` :type "PlayerController Object Reference") (`Character Class` :type "/Game/TPSFPSCharacterSystem/Blueprints/COMMON_CommonCharacter/BP_CommonCharacter Class Reference") (ControllerOnRespawn :type "Controller Object Reference"))
  ;[1 1 1] RespawnPlayerCharacter
  (bind _asbp_common_game_mode (cast `/Game/TPSFPSCharacterSystem/Blueprints/COMMON_GameMode/BP_CommonGameMode` (`GameplayStatics.GetGameMode`)))
  (`/Engine/EditorBlueprintResources/StandardMacros.IsValid` self
    (:`Is Valid`
      (`/Game/TPSFPSCharacterSystem/Blueprints/COMMON_GameMode/BP_CommonGameMode.CharacterRespawn` _asbp_common_game_mode `Player Controller` `Character Class` ControllerOnRespawn)
      (`self.TestMC`))))

(event `TestMC`
  ;[1 1 1] RespawnPlayerCharacter
  (`KismetSystemLibrary.Delay` 4.0)
  (`self.EnableInput` null))

(event `InputAxis|MoveForward` :overrideparent false
  (params (AxisValue :type "Float (single-precision)"))
  ;[1 1 1] MOVE FORWARD
  ;;[1 1 1] InputAxis MoveForward
  (set `self.Initial Move Forward Input Axis Value` AxisValue)
  (`/Engine/EditorBlueprintResources/StandardMacros.IsValid` (`self.GetCommonCharacter`)
    (:`Is Valid`
      ;;[1 1 1] Comment
      (`self.MoveForwardInput`)
      ;;[1 1 1] Sprint Condition
      (if (`/Game/TPSFPSCharacterSystem/Blueprints/COMMON_CommonCharacter/BP_CommonCharacter.GetSprintState` (`self.GetCommonCharacter`))
        ;;[1 1 1] Move in sprint state
        (`|ExecutionSequence`
          (:`then_0`
            (bind _output_get (set `self.Pre Move Forward Axis Value` 1.0)) ; Set max value for sprint move speed
            ;;;[1 1 1] Interpolation
            (set `self.Final Move Forward Axis Value` (`KismetMathLibrary.FInterpTo` (`self.Final Move Forward Axis Value`) _output_get (`GameplayStatics.GetWorldDeltaSeconds`) 10.0))
            ;;;[1 1 1] Add Movement Input
            (`Pawn.AddMovementInput` (`self.K2_GetPawn`) (`self.Forward Vector`) (`self.Final Move Forward Axis Value`) false))
          (:`then_1`
            ;;;[1 1 1] Sprint Off Logic
            (if (<= (`self.Initial Move Forward Input Axis Value`) 0.5)
              (`/Engine/EditorBlueprintResources/StandardMacros.DoOnce` false :!label _label
                (:`Completed`
                  (`self.SprintOff`))))))
        (else
          ;;[1 1 1] Move in stand, crouch and prone states
          (`|ExecutionSequence`
            (:`then_0`
              (goto _label :!via `Reset`))
            (:`then_1`
              (bind _output_get_2 (set `self.Pre Move Forward Axis Value` (`self.Initial Move Forward Input Axis Value`)))
              ;;;[1 1 1] Interpolation
              (set `self.Final Move Forward Axis Value` (`KismetMathLibrary.FInterpTo` (`self.Final Move Forward Axis Value`) _output_get_2 (`GameplayStatics.GetWorldDeltaSeconds`) 10.0))
              ;;;[1 1 1] Add Movement Input
              (`Pawn.AddMovementInput` (`self.K2_GetPawn`) (`self.Forward Vector`) (`self.Final Move Forward Axis Value`) false))))))))

(event `InputAxis|MoveRight` :overrideparent false
  (params (AxisValue :type "Float (single-precision)"))
  ;[1 1 1] MOVE RIGHT
  ;;[1 1 1] InputAxis MoveRight
  (set `self.Initial Move Right Input Axis Value` AxisValue)
  (`/Engine/EditorBlueprintResources/StandardMacros.IsValid` (`self.GetCommonCharacter`)
    (:`Is Valid`
      ;;[1 1 1] Comment
      (`self.MoveRightInput`)
      ;;[1 1 1] Sprint Condition
      (if (`/Game/TPSFPSCharacterSystem/Blueprints/COMMON_CommonCharacter/BP_CommonCharacter.GetSprintState` (`self.GetCommonCharacter`))
        ;;[1 1 1] Move in sptint State
        (bind _output_get (set `self.Pre Move Right Axis Value` (`KismetMathLibrary.FClamp` (`self.Initial Move Right Input Axis Value`) -0.5 0.5)))
        ;;;[1 1 1] Interpolation
        (set `self.Final Move Right Axis Value` (`KismetMathLibrary.FInterpTo` (`self.Final Move Right Axis Value`) _output_get (`GameplayStatics.GetWorldDeltaSeconds`) 10.0))
        ;;;[1 1 1] Add Movement Input
        (`Pawn.AddMovementInput` (`self.K2_GetPawn`) (`self.Right Vector`) (`self.Final Move Right Axis Value`) false)
        (else
          ;;[1 1 1] Move in Stand, crouch and prone state
          (bind _output_get_2 (set `self.Pre Move Right Axis Value` (`self.Initial Move Right Input Axis Value`)))
          ;;;[1 1 1] Interpolation
          (set `self.Final Move Right Axis Value` (`KismetMathLibrary.FInterpTo` (`self.Final Move Right Axis Value`) _output_get_2 (`GameplayStatics.GetWorldDeltaSeconds`) 10.0))
          ;;;[1 1 1] Add Movement Input
          (`Pawn.AddMovementInput` (`self.K2_GetPawn`) (`self.Right Vector`) (`self.Final Move Right Axis Value`) false))))))

(event `InputAxis|LookUp`
  (params (AxisValue :type "Float (single-precision)"))
  ;[1 1 1] LOOK UP
  ;;[1 1 1] Mouse
  ;;;[1 1 1] InputAxis Look Up (MOUSE)
  (set `self.Initial LockUp Mouse Input Axis Value` AxisValue)
  (`/Engine/EditorBlueprintResources/StandardMacros.IsValid` (`self.GetCommonCharacter`)
    (:`Is Valid`
      (`|ExecutionSequence`
        (:`then_0`
          ;;;[1 1 1] Check using mouse
          (if (!= (`self.Initial LockUp Mouse Input Axis Value`) 0.0)
            (set `self.UseMouse?` true)))
        (:`then_1`
          ;;;[1 1 1] Comment
          (`self.LockUpInput`)
          (set `self.Final LockUp Axis Value` (`self.Initial LockUp Mouse Input Axis Value`))
          ;;;[1 1 1] Add Controller Pitch Input
          (`Pawn.AddControllerPitchInput` (`self.K2_GetPawn`) (`self.Final LockUp Axis Value`)))))))

(event `InputAxis|Turn`
  (params (AxisValue :type "Float (single-precision)"))
  ;[1 1 1] TURN
  ;;[1 1 1] Mouse
  ;;;[1 1 1] InputAxis Turn (MOUSE)
  (set `self.Initial Turn Mouse Input Axis Value` AxisValue)
  (`/Engine/EditorBlueprintResources/StandardMacros.IsValid` (`self.GetCommonCharacter`)
    (:`Is Valid`
      (`|ExecutionSequence`
        (:`then_0`
          ;;;[1 1 1] Check using mouse
          (if (!= (`self.Initial Turn Mouse Input Axis Value`) 0.0)
            (set `self.UseMouse?` true)))
        (:`then_1`
          ;;;[1 1 1] Comment
          (`self.TurnInput`)
          ;;;[1 1 1] Prone Condition
          (if (`/Game/TPSFPSCharacterSystem/Blueprints/COMMON_CommonCharacter/BP_CommonCharacter.GetProneState` (`self.GetCommonCharacter`))
            ;;;[1 1 1] Prone
            (set `self.Final Turn Axis Value` (* (`self.Initial Turn Mouse Input Axis Value`) (`self.ProneStateTurnCoeff`)))
            (else
              ;;;[1 1 1] Other State
              (set `self.Final Turn Axis Value` (`self.Initial Turn Mouse Input Axis Value`))))
          ;;;[1 1 1] Add Controller Yaw Input
          (`Pawn.AddControllerYawInput` (`self.K2_GetPawn`) (`self.Final Turn Axis Value`)))))))

(event `InputAxis|TurnRate`
  (params (AxisValue :type "Float (single-precision)"))
  ;[1 1 1] TURN
  ;;[1 1 1] Gamepad
  ;;;[1 1 1] InputAxis Turn (GAMEPAD)
  (set `self.Initial Turn GamePad Input Axis Value` AxisValue)
  (`/Engine/EditorBlueprintResources/StandardMacros.IsValid` (`self.GetCommonCharacter`)
    (:`Is Valid`
      (`|ExecutionSequence`
        (:`then_0`
          ;;;[1 1 1] Check not using mouse
          (if (!= (`self.Initial Turn GamePad Input Axis Value`) 0.0)
            (set `self.UseMouse?` false)))
        (:`then_1`
          ;;;[1 1 1] Comment
          (`/Game/TPSFPSCharacterSystem/Blueprints/COMMON_CommonCharacter/BP_CommonCharacterInterface.TurnInput`)
          ;;;[1 1 1] Set Output Value
          (set `self.Final Turn Axis Value` (* (`self.Initial Turn GamePad Input Axis Value`) 90.0 (`GameplayStatics.GetWorldDeltaSeconds`)))
          ;;;[1 1 1] Add Controller Yaw Input
          (`Pawn.AddControllerYawInput` (`self.K2_GetPawn`) (`self.Final Turn Axis Value`)))))))

(event `InputAxis|LookUpRate`
  (params (AxisValue :type "Float (single-precision)"))
  ;[1 1 1] LOOK UP
  ;;[1 1 1] Gamepad
  ;;;[1 1 1] InputAxis Look Up  (GAMEPAD)
  (set `self.Initial LockUp GamePad Input Axis Value` AxisValue)
  (`/Engine/EditorBlueprintResources/StandardMacros.IsValid` (`self.GetCommonCharacter`)
    (:`Is Valid`
      (`|ExecutionSequence`
        (:`then_0`
          ;;;[1 1 1] Check not using mouse
          (if (!= (`self.Initial LockUp GamePad Input Axis Value`) 0.0)
            (set `self.UseMouse?` false)))
        (:`then_1`
          ;;;[1 1 1] Comment
          (`self.LockUpInput`)
          (set `self.Final LockUp Axis Value` (* (`self.Initial LockUp GamePad Input Axis Value`) 90.0 (`GameplayStatics.GetWorldDeltaSeconds`)))
          ;;;[1 1 1] Add Controller Pitch Input
          (`Pawn.AddControllerPitchInput` (`self.K2_GetPawn`) (`self.Final LockUp Axis Value`)))))))

(fn `GetCommonCharacter`
  (returns (`Common Character` :type "/Game/TPSFPSCharacterSystem/Blueprints/COMMON_CommonCharacter/BP_CommonCharacter Object Reference"))
  (`/Engine/EditorBlueprintResources/StandardMacros.IsValid` (`self.K2_GetPawn`)
    (:`Is Valid`
      (bind _asbp_common_character (cast `/Game/TPSFPSCharacterSystem/Blueprints/COMMON_CommonCharacter/BP_CommonCharacter` (`self.K2_GetPawn`)))
      (return _asbp_common_character))))

(fn `UserConstructionScript`)
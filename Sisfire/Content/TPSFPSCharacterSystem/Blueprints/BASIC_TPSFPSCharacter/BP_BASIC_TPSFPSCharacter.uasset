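; Player character Blueprint that switches between first- and third-person cameras and adds a health bar widget.
; Character state selects BPAdvancedTPSCamera presets, with optional shoulder mirroring in third person.
; Guarded mode switches use timelines to blend spring arm and FOV on one shared camera, then update crosshair, shadows and weapon system through client and server events.
; A debug M key applies heavy damage to the player.
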(event `Key|M`
  (params (Key :type "Key Structure"))
  ;[1 1 1] Kill Player
  (:`Pressed`
    (bind _returnvalue (`GameplayStatics.ApplyDamage` self 1000.0))
    (bind _output_get (set `self.HealthForLifeBar` (- (`self.HealthForLifeBar`) _returnvalue)))
    (`KismetSystemLibrary.PrintString` (`KismetStringLibrary.Conv_DoubleToString` _output_get))))

(event `self.ReceiveBeginPlay`
  ;[1 1 1] EVENT BEGIN PLAY
  (`parent.ReceiveBeginPlay`)
  ;;[1 1 1] InitializeTPSCamera
  (`self.InitializeTPSCamera`)
  ;[1 1 1] Additional Event Play
  (`|ExecutionSequence`
    (:`then_0`
      (bind _returnvalue (`|CreateWidget` "/Game/Nodes/Interactions/HealthBar.HealthBar_C" (`GameplayStatics.GetPlayerController` 0)))
      (`UserWidget.AddToViewport` _returnvalue 0))))

(event `InitializeTPSCamera`
  ;[1 1 1] InitializeTPSCamera
  (`/Engine/EditorBlueprintResources/StandardMacros.IsValid` (`self.BP_AdvancedTPSCamera`)
    (:`Is Valid`
      (`/Engine/EditorBlueprintResources/StandardMacros.IsValid` (`self.SpringArm`)
        (:`Is Valid`
          (`/Engine/EditorBlueprintResources/StandardMacros.IsValid` (`self.FPSCamera`)
            (:`Is Valid`
              (`/Game/TPSFPSCharacterSystem/Blueprints/COMMON_TPSCamera/BP_AdvancedTPSCamera.Set Start Camera Mode` (`self.BP_AdvancedTPSCamera`) (`self.SpringArm`) (`self.FPSCamera`) "FloorIdle" 75.0 -75.0 false))))))))

(event `/Game/TPSFPSCharacterSystem/Blueprints/COMMON_CommonCharacter/BP_CommonCharacterInterface.CharacterStateChanged`
  (params (`Character State` :type "/Game/TPSFPSCharacterSystem/Blueprints/COMMON_CommonCharacter/ENUM_CharacterState Enum" :default "NewEnumerator0"))
  ;[1 1 1] EVENT CHARACTER STATE GHANGED
  (`self.UpdateCameraMode` `Character State`))

(event `/Game/TPSFPSCharacterSystem/Blueprints/COMMON_CommonCharacter/BP_CommonCharacterInterface.CameraMirrow`
  ;[1 1 1] Camera Mirror
  (if (`|EnumEquality` (`self.GetCameraMode`) "NewEnumerator1")
    (if (not (`self.GetInChangingCameraMode`))
      (if (`self.Camera Mirror?`)
        (set `self.Camera Mirror?` false)
        (else
          (set `self.Camera Mirror?` true)))
      (`/Game/TPSFPSCharacterSystem/Blueprints/COMMON_TPSCamera/BP_AdvancedTPSCamera.OpenGateChange` (`self.BP_AdvancedTPSCamera`))
      (`self.ChangeTPSCameraState` (`/Game/TPSFPSCharacterSystem/Blueprints/COMMON_TPSCamera/BP_AdvancedTPSCamera.Current Camera Mode` (`self.BP_AdvancedTPSCamera`))))))

(event `UpdateCameraMode`
  (params (`Character State` :type "/Game/TPSFPSCharacterSystem/Blueprints/COMMON_CommonCharacter/ENUM_CharacterState Enum" :default "NewEnumerator0"))
  ;[1 1 1] UpdateCameraMode
  (if (`|EnumEquality` (`self.GetCameraMode`) "NewEnumerator1")
    (if (not (`self.GetInChangingCameraMode`))
      (switch `/Game/TPSFPSCharacterSystem/Blueprints/COMMON_CommonCharacter/ENUM_CharacterState` `Character State`
        (:`NewEnumerator0`
          (`self.ChangeTPSCameraState` "FloorIdle"))
        (:`NewEnumerator1`
          (`self.ChangeTPSCameraState` "FloorMiniZoom"))
        (:`NewEnumerator2`
          (`self.ChangeTPSCameraState` "CrouchIdle"))
        (:`NewEnumerator3`
          (`self.ChangeTPSCameraState` "CrouchMiniZoom"))
        (:`NewEnumerator6`
          (`self.ChangeTPSCameraState` "FloorSprint"))
        (:`NewEnumerator7`
          (`self.ChangeTPSCameraState` "CrouchIdle" :!label _label))
        (:`NewEnumerator8`
          (goto _label))))))

(event `/Game/TPSFPSCharacterSystem/Blueprints/COMMON_CommonCharacter/BP_CommonCharacterInterface.SwitchTPSFPSCameraMode`
  ;[1 1 1] SWITCH TPS FPS CAMERA MODE / FIRE FROM PLAYER CONTROLLER
  (`self.ChangeCameraMode`))

(event `ServerUpdateOnChangeCameraModeToFPS`
  ;[1 1 1] ServerUpdateOnChangeCameraModeToFPS / TPS
  (`/Game/TPSFPSCharacterSystem/Blueprints/COMMON_WeaponSystem/BP_WeaponSystem.MulticastUpdateInFPSChar` (`self.BP_WeaponSystem`) true)
  ;[1 0 0] Add
  (`self.SetCameraMode` "NewEnumerator0"))

(event `ClientUpdateOnChangeCameraMode`
  ;[1 1 1] ClientUpdateOnChangeCameraMode
  (switch `/Game/TPSFPSCharacterSystem/Blueprints/BASIC_FPSCharacter/Data/ENUM_BASIC_FPS_TPS_CAM_MODE` (`self.GetCameraMode`)
    (:`NewEnumerator0`
      (`self.ServerUpdateOnChangeCameraModeToFPS`)
      ;[1 0 0] FixShadows
      (`self.FixShadows` false))
    (:`NewEnumerator1`
      (`self.ServerUpdateOnChangeCameraModeToTPS`)
      (`self.FixShadows` true))))

(event `ServerUpdateOnChangeCameraModeToTPS`
  ;[1 1 1] ServerUpdateOnChangeCameraModeToFPS / TPS
  (`/Game/TPSFPSCharacterSystem/Blueprints/COMMON_WeaponSystem/BP_WeaponSystem.MulticastUpdateInFPSChar` (`self.BP_WeaponSystem`) false)
  ;[1 0 0] Add
  (`self.SetCameraMode` "NewEnumerator1"))

(event `ChangeCameraMode`
  (bind (_targetarmlength _socketoffset _targetoffset _fieldofview) (`self.GetCameraState`))
  (bind (_in_fps_cam_changing_fov_ _in_fps_cam_changing_position_) (`self.GetFPSCamStates`))
  (bind (_targetarmlength_2 _socketoffset_2 _targetoffset_2 _fieldofview_2) (`self.GetCameraState`))
  (bind _bp_weaponsystem (`self.BP_WeaponSystem`))
  ;[1 1 1] ChangeCameraMode
  ;;[1 1 1] Conditions for chanding camera mode
  (if (`self.GetInChangingCameraMode`)
    _
    (elif (`/Game/TPSFPSCharacterSystem/Blueprints/COMMON_TPSCamera/BP_AdvancedTPSCamera.Get In Transition Between Presets` (`self.BP_AdvancedTPSCamera`))
      _
      (elif (not (or _in_fps_cam_changing_fov_ _in_fps_cam_changing_position_))
        ;;[1 1 1] Set State In Changing Camera Mode
        (`self.SetInChangingCameraMode` true)
        ;;[1 1 1] Check Current Camera Mode
        (switch `/Game/TPSFPSCharacterSystem/Blueprints/BASIC_FPSCharacter/Data/ENUM_BASIC_FPS_TPS_CAM_MODE` (`self.GetCameraMode`)
          (:`NewEnumerator0`
            ;;[1 1 1] TO TPS MODE
            ;;;[1 1 1] ReSet Basic Setting
            (`self.SetCameraMode` "NewEnumerator1")
            (`self.GoThierPersonView`)
            (`self.UpdateUsePawnControlRotationSetting`)
            ;;;[1 1 1] Set FPS CAMERA Rotation == 0
            (`SceneComponent.K2_SetRelativeRotation` :`self` (`self.FPSCamera`))
            ;;;[1 1 1] Define Current Preset for TPS MODE
            (`self.DefineTPSCameraTransferPreset`)
            ;;;[1 1 1] Crosshair Logic
            (`/Game/TPSFPSCharacterSystem/Blueprints/COMMON_WeaponSystem/BP_WeaponSystem.ShowMainpartCrossHair` _bp_weaponsystem)
            (`/Game/TPSFPSCharacterSystem/Blueprints/COMMON_WeaponSystem/BP_WeaponSystem.ShowCrossHair` _bp_weaponsystem)
            ;;;[1 1 1] Smooth Transition
            (bind (_direction _updated_coeff) (`Timeline|ChangeCameraModeFPStoTPS` :!via `PlayFromStart`)
              (:`Update`
                (bind (_targetarmlength_3 _socketoffset_3 _targetoffset_3 _fov) (`/Game/TPSFPSCharacterSystem/Blueprints/COMMON_TPSCamera/BP_AdvancedTPSCamera.GetCameraSettingsFromPreset` (`self.BP_AdvancedTPSCamera`) (`self.TransferTPSCameraName`)))
                (`self.SetCameraState` (`|EaseFunction` "Linear" _updated_coeff _targetarmlength_2 _targetarmlength_3) (`|EaseFunction` "Linear" _updated_coeff _socketoffset_2 _socketoffset_3) (`|EaseFunction` "Linear" _updated_coeff _targetoffset_2 _targetoffset_3) (`|EaseFunction` "Linear" _updated_coeff _fieldofview_2 _fov)))
              (:`Finished`
                (`/Game/TPSFPSCharacterSystem/Blueprints/COMMON_TPSCamera/BP_AdvancedTPSCamera.SetCurrentCameraPreset` (`self.BP_AdvancedTPSCamera`) (`self.TransferTPSCameraName`))
                (`self.SetInChangingCameraMode` false)
                (`self.ClientUpdateOnChangeCameraMode`))))
          (:`NewEnumerator1`
            ;;[1 1 1] TO FPS MODE
            ;;;[1 1 1] ReSet Basic Setting
            (`self.SetCameraMode` "NewEnumerator0")
            (`self.DefineFPSCameraSetting`)
            ;;;[1 1 1] Smooth Transition
            (bind (_direction_2 _updated_coeff_2) (`Timeline|ChangeCameraModeTPStoFPS` :!via `PlayFromStart`)
              (:`Update`
                (`|ExecutionSequence`
                  (:`then_0`
                    (if (>= _updated_coeff_2 0.8)
                      (`/Engine/EditorBlueprintResources/StandardMacros.DoOnce` false :!label _label_2
                        (:`Completed`
                          ;;;[1 1 1] ReSet Basic Setting
                          (`self.GoFirstPersonView`)
                          (`self.UpdateUsePawnControlRotationSetting`)
                          ;;;[1 1 1] Crosshair Logic
                          (`/Game/TPSFPSCharacterSystem/Blueprints/COMMON_WeaponSystem/BP_WeaponSystem.ShowHideCrossHairInAimMode` (`self.BP_WeaponSystem`) (`self.GetAimStates`))))))
                  (:`then_1`
                    (`self.SetCameraState` (`|EaseFunction` "Linear" _updated_coeff_2 _targetarmlength) (`|EaseFunction` "Linear" _updated_coeff_2 _socketoffset (`self.SocketOffSet FPS Camera`)) (0.0 0.0 0.0) (`|EaseFunction` "Linear" _updated_coeff_2 _fieldofview (`self.FPS Camera FOV`))))))
              (:`Finished`
                (`self.SetInChangingCameraMode` false)
                (`self.ClientUpdateOnChangeCameraMode`)
                (goto _label_2 :!via `Reset`)))))))))

(fn `ChangeTPSCameraState`
  (params (`Input Camera Preset` :type Name))
  (`/Game/TPSFPSCharacterSystem/Blueprints/COMMON_TPSCamera/BP_AdvancedTPSCamera.OpenGateChange` (`self.BP_AdvancedTPSCamera`))
  (`/Game/TPSFPSCharacterSystem/Blueprints/COMMON_TPSCamera/BP_AdvancedTPSCamera.Change Camera Mode` (`self.BP_AdvancedTPSCamera`) (`self.SpringArm`) (`self.FPSCamera`) `Input Camera Preset` (`self.Camera Mirror?`)))

(fn `DefineFPSCameraSetting`
  (bind (_crouchcamerazlocation _floorcamerazlocation _camera_default_fov) (`self.GetFPSCameraSetting`))
  (bind (_crouchcamerazlocation_2 _floorcamerazlocation_2 _camera_default_fov_2) (`self.GetFPSCameraSetting`))
  (bind (_crouchcamerazlocation_3 _floorcamerazlocation_3 _camera_default_fov_3 _camera_aim_fov) (`self.GetFPSCameraSetting`))
  (bind (_crouchcamerazlocation_4 _floorcamerazlocation_4 _camera_default_fov_4 _camera_aim_fov_2) (`self.GetFPSCameraSetting`))
  (if (`self.GetCrouchState`)
    (if (`self.GetAimStates`)
      (set `self.SocketOffSet FPS Camera` (`KismetMathLibrary.MakeVector` 0.0 0.0 _crouchcamerazlocation_4))
      (set `self.FPS Camera FOV` _camera_aim_fov_2)
      (else
        (set `self.SocketOffSet FPS Camera` (`KismetMathLibrary.MakeVector` 0.0 0.0 _crouchcamerazlocation))
        (set `self.FPS Camera FOV` _camera_default_fov)))
    (elif (`self.GetAimStates`)
      (set `self.SocketOffSet FPS Camera` (`KismetMathLibrary.MakeVector` 0.0 0.0 _floorcamerazlocation_3))
      (set `self.FPS Camera FOV` _camera_aim_fov)
      (else
        (set `self.SocketOffSet FPS Camera` (`KismetMathLibrary.MakeVector` 0.0 0.0 _floorcamerazlocation_2))
        (set `self.FPS Camera FOV` _camera_default_fov_2)))))

(fn `DefineTPSCameraTransferPreset`
  (switch `/Game/TPSFPSCharacterSystem/Blueprints/COMMON_CommonCharacter/ENUM_CharacterState` (`self.GetMainCharacterState`)
    (:`NewEnumerator0`
      (set `self.TransferTPSCameraName` "FloorIdle"))
    (:`NewEnumerator1`
      (set `self.TransferTPSCameraName` "FloorMiniZoom"))
    (:`NewEnumerator2`
      (set `self.TransferTPSCameraName` "CrouchIdle"))
    (:`NewEnumerator3`
      (set `self.TransferTPSCameraName` "CrouchMiniZoom"))
    (:`NewEnumerator6`
      (set `self.TransferTPSCameraName` "FloorSprint"))
    (:`NewEnumerator7`
      (set `self.TransferTPSCameraName` "CrouchIdle" :!label _label))
    (:`NewEnumerator8`
      (goto _label))))

(fn `GetCameraState`
  (returns (TargetArmLength :type "Float (double-precision)") (SocketOffset :type "Vector Structure") (TargetOffset :type "Vector Structure") (FieldOfView :type "Float (double-precision)"))
  (bind _springarm (`self.SpringArm`))
  (bind _fpscamera (`self.FPSCamera`))
  (`/Engine/EditorBlueprintResources/StandardMacros.IsValid` _springarm
    (:`Is Valid`
      (`/Engine/EditorBlueprintResources/StandardMacros.IsValid` _fpscamera
        (:`Is Valid`
          (return (`SpringArmComponent.TargetArmLength` _springarm) (`SpringArmComponent.SocketOffset` _springarm) (`SpringArmComponent.TargetOffset` _springarm) (`CameraComponent.FieldOfView` _fpscamera)))))))

(fn `SetCameraState`
  (params (TargetArmLength :type "Float (double-precision)") (SocketOffset :type "Vector Structure") (TargetOffset :type "Vector Structure") (FieldOfView :type "Float (double-precision)"))
  (bind _springarm (`self.SpringArm`))
  (bind _fpscamera (`self.FPSCamera`))
  (`/Engine/EditorBlueprintResources/StandardMacros.IsValid` _springarm
    (:`Is Valid`
      (`/Engine/EditorBlueprintResources/StandardMacros.IsValid` _fpscamera
        (:`Is Valid`
          (set `SpringArmComponent.TargetArmLength` TargetArmLength _springarm)
          (set `SpringArmComponent.SocketOffset` SocketOffset _springarm)
          (set `SpringArmComponent.TargetOffset` TargetOffset _springarm)
          (set `CameraComponent.FieldOfView` FieldOfView _fpscamera))))))

(fn `UpdateUsePawnControlRotationSetting`
  (switch `/Game/TPSFPSCharacterSystem/Blueprints/BASIC_FPSCharacter/Data/ENUM_BASIC_FPS_TPS_CAM_MODE` (`self.GetCameraMode`)
    (:`NewEnumerator0`
      (set `SpringArmComponent.bUsePawnControlRotation` false (`self.SpringArm`))
      (set `CameraComponent.bUsePawnControlRotation` true (`self.FPSCamera`)))
    (:`NewEnumerator1`
      (set `SpringArmComponent.bUsePawnControlRotation` true (`self.SpringArm`))
      (set `CameraComponent.bUsePawnControlRotation` false (`self.FPSCamera`)))))

(fn `UserConstructionScript`
  (`parent.UserConstructionScript`))
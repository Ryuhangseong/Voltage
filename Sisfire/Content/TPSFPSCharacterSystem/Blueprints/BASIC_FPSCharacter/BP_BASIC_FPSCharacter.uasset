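; Basic FPS character Blueprint that adds first-person camera and weapon handling to its parent, with FPS/TPS camera modes.
; Authority spawns primary and secondary weapons; swaps and pickups re-attach the current weapon, reinitialise weapon system and shoot animations, and update HUD and shadows.
; Weapons snap to first-person arms for the local FPS player, otherwise to the body mesh.
; Timer-stepped FOV handles aiming, timelines handle crouch height, and death switches to third-person view.
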(event `self.ReceiveBeginPlay`
  ;[1 1 1] EVENT BEGIN PLAY (ON SPAWN CHARACTER)
  (`parent.ReceiveBeginPlay`)
  ;;[1 1 1] Initialize FPS Camera
  (`self.InitializeFPSCamera`)
  (`|ExecutionSequence`
    (:`then_0`
      (`/Engine/EditorBlueprintResources/ActorMacros.Switch Has Authority`
        (:`Authority`
          ;;[1 1 1] Spawn Base Weapon as Primary Weapon
          (bind _returnvalue (`|SpawnActorFromClass` (`self.PrimaryWeaponClass`) (`SceneComponent.GetRelativeTransform` (`self.Mesh`)) "AlwaysSpawn" "SelectDefaultAtRuntime" null null))
          (`/Engine/EditorBlueprintResources/StandardMacros.IsValid` _returnvalue
            (:`Is Valid`
              (`self.Set Primary Weapon Actor` _returnvalue)
              ;;[1 1 1] Spawn Base Weapon as Secondary Weapon
              (bind _returnvalue_2 (`|SpawnActorFromClass` (`self.SecondaryWeaponClass`) (`SceneComponent.GetRelativeTransform` (`self.Mesh`)) "AlwaysSpawn" "SelectDefaultAtRuntime" null null))
              (`/Engine/EditorBlueprintResources/StandardMacros.IsValid` _returnvalue_2
                (:`Is Valid`
                  (`self.Set Secondary Weapon Actor` _returnvalue_2)
                  ;;[1 1 1] Set Hiden Secondary Weapon & Set Primary Slot in Hand
                  (`self.SetActorHiddenInGame` (`self.Get Secondary Weapon Actor`) false)
                  (`self.Set Current Weapon Slot In Hand` "NewEnumerator0")
                  ;;[1 1 1] Initialize Basic FPS Weapon
                  (`self.Initialize Base FPS Weapon`)
                  (`self.ClientUpdateHUDWeaponProp`))))))
        (:`Remote`
          ;;[1 0 0] Trigger FixShadows
          (`self.FixShadows` false)
          ;;[1 1 1] ClientAttachWeapon
          (`KismetSystemLibrary.Delay` 1.0)
          (`self.ClientAttachWeapon`)
          ;;[1 1 1] Comment
          (bind _asbp_basic_wpn_base_weapon (cast `/Game/TPSFPSCharacterSystem/Blueprints/BASIC_BaseCharacter/Data/BP_BASIC_WPN_BaseWeapon` (`self.Get Current Base Weapon`) :!label _label))
          (`self.SetPlayerHUDProperties` (`/Game/TPSFPSCharacterSystem/Blueprints/BASIC_BaseCharacter/Data/BP_BASIC_WPN_BaseWeapon.HUD Properties` _asbp_basic_wpn_base_weapon)))))
    (:`then_1`
      ;;[1 1 1] Wait basic logics
      (`KismetSystemLibrary.Delay` 1.0)
      ;;[1 1 1] Attach Current Weapon
      (`self.Attach Current Weapon` (`self.Get Current Base Weapon`))
      (`self.ClientAttachWeapon`))))

(event `ClientUpdateHUDWeaponProp`
  ;[1 1 1] EVENT BEGIN PLAY (ON SPAWN CHARACTER)
  ;;[1 1 1] Comment
  (goto _label))

(event `InitializeFPSCamera`
  (bind _returnvalue (`GameplayStatics.GetPlayerCameraManager` 0))
  ;[1 1 1] InitializeFPSCamera
  ;;[1 1 1] View Pitch Angels
  (set `PlayerCameraManager.ViewPitchMax` 75.0 _returnvalue)
  (set `PlayerCameraManager.ViewPitchMin` -75.0 _returnvalue)
  ;;[1 1 1] FOV
  (set `self.CurrentFPSCameraFOV` (`self.Camera Default FOV`)))

(event `ClientAttachWeapon`
  ;[1 1 1] ClientAttachWeapon
  (`self.Attach Current Weapon` (`self.Get Current Base Weapon`)))

(event `MulticastAttacthWeapon`
  ;[1 1 1] MulticastAttacthWeapon
  ;;[1 1 1] Attach Current Weapon
  (`self.Attach Current Weapon` (`self.Get Current Base Weapon`)))

(event `/Game/TPSFPSCharacterSystem/Blueprints/COMMON_CommonCharacter/BP_CommonCharacterInterface.SwapTriggerFire`
  ;[1 1 1] Swap
  (`self.MulticastAttacthWeapon` :!label _label_2)
  (`KismetSystemLibrary.Delay` 0.2)
  (`self.MulticastAttacthWeapon`)
  (`self.ClientAttachWeapon`)
  ;;[1 1 1] Interface Call - Weapon Is Attached
  (`/Game/TPSFPSCharacterSystem/Blueprints/COMMON_CommonCharacter/BP_CommonCharacterInterface.WeaponIsAttached`)
  ;;[1 1 1] Initialize FPS Weapon
  (`self.Initialize Base FPS Weapon`)
  (`self.ClientUpdateHUDWeaponProp`)
  ;[1 0 0] Trigger FixShadows
  (switch `/Game/TPSFPSCharacterSystem/Blueprints/BASIC_FPSCharacter/Data/ENUM_BASIC_FPS_TPS_CAM_MODE` (`self.Camera Mode`)
    (:`NewEnumerator0`
      (`self.FixShadows` false))
    (:`NewEnumerator1`
      (`self.FixShadows` true))))

(event `/Game/TPSFPSCharacterSystem/Blueprints/COMMON_CommonCharacter/BP_CommonCharacterInterface.AimStateChanged`
  (params (`Aim?` :type Boolean))
  ;[1 1 1] Event Character State Changed
  ;;[1 1 1] FPS CAM CONTROLLER
  (`self.UpdateFPSCameraAimFOV` `Aim?`))

(event `/Game/TPSFPSCharacterSystem/Blueprints/COMMON_CommonCharacter/BP_CommonCharacterInterface.WeaponPickuped`
  ;[1 1 1] Swap
  (goto _label_2))

(event `FixShadows`
  (params (`Shadows On` :type Boolean))
  (bind (_current_weapon _currentweaponslotinhand) (`self.Get Current Base Weapon`))
  ;[1 0 0] FixShadows
  (`/Engine/EditorBlueprintResources/StandardMacros.IsValid` (`self.Get Current Base Weapon`)
    (:`Is Valid`
      (`PrimitiveComponent.SetCastShadow` (`/Game/TPSFPSCharacterSystem/Blueprints/COMMON_WeaponSystem/BP_BaseWeapon.WeaponSkeletalMesh` _current_weapon) `Shadows On`)
      (switch `/Game/TPSFPSCharacterSystem/Blueprints/COMMON_CommonCharacter/ENUM_CharacterWeaponSlot` _currentweaponslotinhand
        (:`NewEnumerator0`
          (`/Engine/EditorBlueprintResources/StandardMacros.IsValid` (`self.Get Base Secondary Weapon`)
            (:`Is Valid`
              (if `Shadows On`
                (`PrimitiveComponent.SetCastShadow` (`/Game/TPSFPSCharacterSystem/Blueprints/COMMON_WeaponSystem/BP_BaseWeapon.WeaponSkeletalMesh` (`self.Get Base Secondary Weapon`)) false)
                (else
                  (`PrimitiveComponent.SetCastShadow` (`/Game/TPSFPSCharacterSystem/Blueprints/COMMON_WeaponSystem/BP_BaseWeapon.WeaponSkeletalMesh` (`self.Get Base Secondary Weapon`)) false))))))
        (:`NewEnumerator1`
          (`/Engine/EditorBlueprintResources/StandardMacros.IsValid` (`self.Get Base Primary Weapon`)
            (:`Is Valid`
              (if `Shadows On`
                (`PrimitiveComponent.SetCastShadow` (`/Game/TPSFPSCharacterSystem/Blueprints/COMMON_WeaponSystem/BP_BaseWeapon.WeaponSkeletalMesh` (`self.Get Base Primary Weapon`)) false)
                (else
                  (`PrimitiveComponent.SetCastShadow` (`/Game/TPSFPSCharacterSystem/Blueprints/COMMON_WeaponSystem/BP_BaseWeapon.WeaponSkeletalMesh` (`self.Get Base Primary Weapon`)) false))))))))))

(event `/Game/TPSFPSCharacterSystem/Blueprints/COMMON_CommonCharacter/BP_CommonCharacterInterface.CrouchStateChanged`
  (params (`In Crouch?` :type Boolean))
  ;[1 1 1] Event Character State Changed
  ;;[1 1 1] FPS CAM CONTROLLER
  (`self.UpdateFPSCameraPosition` `In Crouch?`))

(event `/Game/TPSFPSCharacterSystem/Blueprints/COMMON_CommonCharacter/BP_CommonCharacterInterface.DeadStateChanged`
  (params (`In Dead?` :type Boolean))
  ;[1 1 1] Event Character State Changed
  (if `In Dead?`
    ;;[1 1 1] FPS CAM CONTROLLER
    (`self.ClientTriggerActivateDeathCamera`)))

(event `ClientTriggerActivateDeathCamera`
  ;[1 1 1] Event Character State Changed
  (if (`|EnumEquality` (`self.Camera Mode`) "NewEnumerator0")
    (`self.GoThierPersonView`)
    (set `SpringArmComponent.TargetArmLength` 300.0 (`self.SpringArm`))
    (`SceneComponent.K2_SetRelativeLocation` (`self.SpringArm`) (0.0 0.0 -80.0) false false)
    (`Controller.SetControlRotation` (`GameplayStatics.GetPlayerController` 0) (`KismetMathLibrary.MakeRotator` 0.0))))

(event `UpdateFPSCameraAimFOV`
  (params (`Aim?` :type Boolean))
  (if (`|EnumEquality` (`self.Camera Mode`) "NewEnumerator0")
    ;[1 1 1] WS - Show Hide Cross Hair in Aim
    (`/Game/TPSFPSCharacterSystem/Blueprints/COMMON_WeaponSystem/BP_WeaponSystem.ShowHideCrossHairInAimMode` (`self.BP_WeaponSystem`) `Aim?`)
    ;[1 1 1] CALL ON INTERFACE EVENT /// UpdateFPSCameraAimFOV
    (if (not (`self.GetInChangingCameraMode`))
      ;[1 1 1] FOV
      (set `self.In FPS Cam Changing FOV?` true)
      (if `Aim?`
        (`self.StartChanging FPSCameraFOV`)
        (else
          (`self.StartChanging FPSCameraFOV`))))))

(event `StartChanging FPSCameraFOV`
  ;[1 1 1] FOV
  ;;[1 1 1] StartChanging FPSCameraFOV
  (`self.StopChanging FPSCameraFOV`)
  ;;;[1 1 1] Calculation InterpolationTimeStep
  (set `self.InterpolationTimeStep` (/ (`/Game/TPSFPSCharacterSystem/Blueprints/COMMON_WeaponSystem/BP_WeaponSystem.GetWeaponAimRate` (`self.BP_WeaponSystem`)) (`KismetMathLibrary.Conv_IntToDouble` (`self.ChangeFOVInterpolationStepCount`))))
  (if (`self.GetAimStates`)
    ;;;[1 1 1] Main to Aim  /// Interpolation Step Calculation
    (set `self.InterpolationStep` (/ (- (`self.Camera Aim FOV`) (`self.CurrentFPSCameraFOV`)) (`KismetMathLibrary.Conv_IntToDouble` (`self.ChangeFOVInterpolationStepCount`))))
    (else
      ;;;[1 1 1] Aim to Main /// Interpolation Step Calculation
      (set `self.InterpolationStep` (/ (- (`self.Camera Default FOV`) (`self.CurrentFPSCameraFOV`)) (`KismetMathLibrary.Conv_IntToDouble` (`self.ChangeFOVInterpolationStepCount`))))))
  ;;;[1 1 1] Call StepChanging FPSCameraFOV
  (`self.StepChanging FPSCameraFOV`)
  (`KismetSystemLibrary.K2_SetTimer` null "StepChanging FPSCameraFOV" (`self.InterpolationTimeStep`) true))

(event `StopChanging FPSCameraFOV`
  ;[1 1 1] FOV
  ;;[1 1 1] StopChanging FPSCameraFOV
  (`KismetSystemLibrary.K2_ClearTimer` null "StepChanging FPSCameraFOV")
  (set `self.InterpolationStep` 0.0))

(event `StepChanging FPSCameraFOV`
  ;[1 1 1] FOV
  ;;[1 1 1] StepChanging FPSCameraFOV
  (if (`self.GetAimStates`)
    ;;;[1 1 1] Main to Aim Condition
    (if (`KismetMathLibrary.NearlyEqual_FloatFloat` (`self.CurrentFPSCameraFOV`) (`self.Camera Aim FOV`) 1.0)
      ;;;[1 1 1] Stop // FOV == AIM
      (`self.StopChanging FPSCameraFOV`)
      (set `CameraComponent.FieldOfView` (`self.Camera Aim FOV`) (`self.FPSCamera`))
      (set `self.In FPS Cam Changing FOV?` false)
      (else
        ;;;[1 1 1] Step Calculation
        (bind _output_get (set `self.CurrentFPSCameraFOV` (+ (`self.CurrentFPSCameraFOV`) (`self.InterpolationStep`)) :!label _label))
        (set `CameraComponent.FieldOfView` _output_get (`self.FPSCamera`))))
    (else
      ;;;[1 1 1] Aim to Main Condition
      (if (`KismetMathLibrary.NearlyEqual_FloatFloat` (`self.CurrentFPSCameraFOV`) (`self.Camera Default FOV`) 1.0)
        ;;;[1 1 1] Stop // FOV == MAIN
        (`self.StopChanging FPSCameraFOV`)
        (set `CameraComponent.FieldOfView` (`self.Camera Default FOV`) (`self.FPSCamera`))
        (set `self.In FPS Cam Changing FOV?` false)
        (else
          (goto _label))))))

(event `UpdateFPSCamSprintArmLength`
  (params (`In Dead State?` :type Boolean))
  ;[1 1 1] UpdateFPSCamSprintArmLength
  (if (`|EnumEquality` (`self.Camera Mode`) "NewEnumerator0")
    (if (`self.GetInChangingCameraMode`)
      _
      (elif `In Dead State?`
        (`|ExecutionSequence`
          (:`then_0`
            (bind (_direction _newtrack_0) (`Timeline|SptingArmMainToDeadState` :!via `PlayFromStart` :!label _label_2)
              (:`Update`
                (set `SpringArmComponent.TargetArmLength` (`|EaseFunction` "Linear" _newtrack_0 (`SpringArmComponent.TargetArmLength` (`self.SpringArm`)) 300.0) (`self.SpringArm`))))))
        (else
          (`|ExecutionSequence`
            (:`then_1`
              (goto _label_2 :!via `Stop`))))))))

(event `UpdateFPSCameraPosition`
  (params (`Crouch?` :type Boolean))
  ;[1 1 1] CROUCH POSITION
  (if (`|EnumEquality` (`self.Camera Mode`) "NewEnumerator0")
    (if (not (`self.GetInChangingCameraMode`))
      (set `self.In FPS Cam Changing Position?` true)
      (if `Crouch?`
        (`|ExecutionSequence`
          (:`then_0`
            ;;[1 1 1] to crouch
            (bind (_direction _newtrack_0) (`Timeline|ToStandTimeLine` :!via `PlayFromStart` :!label _label_3)
              (:`Update`
                (set `SpringArmComponent.SocketOffset` (`KismetMathLibrary.MakeVector` 0.0 0.0 (`|EaseFunction` "Linear" _newtrack_0 (.z (`SpringArmComponent.SocketOffset` (`self.SpringArm`))) (`self.CrouchCameraZLocation`))) (`self.SpringArm`)))
              (:`Finished`
                (set `self.In FPS Cam Changing Position?` false))))
          (:`then_1`
            ;;[1 1 1] from crouch
            (bind (_direction_2 _newtrack_0_2) (`Timeline|ToCrouchTimeLine` :!via `Stop` :!label _label_4)
              (:`Update`
                (set `SpringArmComponent.SocketOffset` (`KismetMathLibrary.MakeVector` 0.0 0.0 (`|EaseFunction` "Linear" _newtrack_0_2 (.z (`SpringArmComponent.SocketOffset` (`self.SpringArm`))) (`self.FloorCameraZLocation`))) (`self.SpringArm`)))
              (:`Finished`
                (set `self.In FPS Cam Changing Position?` false)))))
        (else
          (`|ExecutionSequence`
            (:`then_0`
              (goto _label_4 :!via `PlayFromStart`))
            (:`then_1`
              (goto _label_3 :!via `Stop`))))))))

(fn `Attach Current Weapon`
  (params (`Current Weapon` :type "Actor Object Reference"))
  (`/Engine/EditorBlueprintResources/StandardMacros.IsValid` `Current Weapon`
    (:`Is Valid`
      (if (`|EnumEquality` (`self.Camera Mode`) "NewEnumerator0")
        (`self.K2_AttachToComponent` `Current Weapon` (select `bool` (`self.IsLocallyControlled`) :`false` (`self.Mesh`) :`true` (`self.1stPPArms`)) "VB WeaponSnap" "SnapToTarget" "KeepRelative" "KeepRelative" true)
        (else
          (`self.K2_AttachToComponent` `Current Weapon` (`self.Mesh`) "VB WeaponSnap" "SnapToTarget" "KeepRelative" "KeepRelative" true))))))

(fn `GetCameraMode`
  (returns (`Camera Mode` :type "/Game/TPSFPSCharacterSystem/Blueprints/BASIC_FPSCharacter/Data/ENUM_BASIC_FPS_TPS_CAM_MODE Enum"))
  (return (`self.Camera Mode`)))

(fn `GetFPSCameraSetting`
  (returns (CrouchCameraZLocation :type "Float (double-precision)") (FloorCameraZLocation :type "Float (double-precision)") (`Camera Default FOV` :type "Float (double-precision)") (`Camera Aim FOV` :type "Float (double-precision)"))
  (return (`self.CrouchCameraZLocation`) (`self.FloorCameraZLocation`) (`self.Camera Default FOV`) (`self.Camera Aim FOV`)))

(fn `GetFPSCamStates`
  (returns (`In FPS Cam Changing FOV?` :type Boolean) (`In FPS Cam Changing Position?` :type Boolean))
  (return (`self.In FPS Cam Changing FOV?`) (`self.In FPS Cam Changing Position?`)))

(fn `GetInChangingCameraMode`
  (returns (`In Changing Camera Mode?` :type Boolean))
  (return (`self.In Changing Camera Mode?`)))

(fn `GoFirstPersonView`
  (`PrimitiveComponent.SetOwnerNoSee` (`self.1stPPArms`) false)
  (`PrimitiveComponent.SetOwnerNoSee` (`self.Mesh`) true)
  (`self.K2_AttachToComponent` (`self.Get Current Base Weapon`) (`self.1stPPArms`) "VB WeaponSnap" "SnapToTarget" "KeepRelative" "KeepRelative" true)
  (`/Game/TPSFPSCharacterSystem/Blueprints/COMMON_WeaponSystem/BP_WeaponSystem.ShowCrossHair` (`self.BP_WeaponSystem`)))

(fn `GoThierPersonView`
  (`PrimitiveComponent.SetOwnerNoSee` (`self.1stPPArms`) true)
  (`PrimitiveComponent.SetOwnerNoSee` (`self.Mesh`) false)
  (`self.K2_AttachToComponent` (`self.Get Current Base Weapon`) (`self.Mesh`) "VB WeaponSnap" "SnapToTarget" "KeepRelative" "KeepRelative" true)
  (`/Game/TPSFPSCharacterSystem/Blueprints/COMMON_WeaponSystem/BP_WeaponSystem.HideCrossHair` (`self.BP_WeaponSystem`)))

(fn `Initialize Base FPS Weapon`
  (locals (loc_row :type "/Game/TPSFPSCharacterSystem/Blueprints/BASIC_FPSCharacter/Data/STR_BASIC_FPS_WeaponDecs Structure"))
  ;[0.2017 1 0.05392] WS Set Current Weapon
  (`/Game/TPSFPSCharacterSystem/Blueprints/COMMON_WeaponSystem/BP_WeaponSystem.SetCurrentWeapon` (`self.BP_WeaponSystem`) (`self.Get Current Base Weapon`))
  ;[1 1 1] Initialize basic base settings
  (bind _asbp_basic_wpn_base_weapon (cast `/Game/TPSFPSCharacterSystem/Blueprints/BASIC_BaseCharacter/Data/BP_BASIC_WPN_BaseWeapon` (`self.Get Current Base Weapon`)))
  (bind (_weaponpositioninrighthand _usedefaultreloadanimation_ _newreloadanimationmontage) (break `/Game/TPSFPSCharacterSystem/Blueprints/BASIC_BaseCharacter/Data/STR_BASIC_Weapon3RDPPPropertiesDesc` (`/Game/TPSFPSCharacterSystem/Blueprints/BASIC_BaseCharacter/Data/BP_BASIC_WPN_BaseWeapon.Get3RDPPProperties` _asbp_basic_wpn_base_weapon)))
  (`self.Initialize Basic Base Properties` (`.WeaponAnimType_2_A75BFA7B422FB26C78E0AEB118FABFDD` (break `/Game/TPSFPSCharacterSystem/Blueprints/BASIC_BaseCharacter/Data/STR_BASIC_WeaponCommonPropertiesDesc` (`/Game/TPSFPSCharacterSystem/Blueprints/BASIC_BaseCharacter/Data/BP_BASIC_WPN_BaseWeapon.GetCommonProperties` _asbp_basic_wpn_base_weapon))) _weaponpositioninrighthand _usedefaultreloadanimation_ _newreloadanimationmontage)
  ;[1 1 1] Shooting Animation Controller
  (bind _asbp_basic_wpn_fps_base_weapon (cast `/Game/TPSFPSCharacterSystem/Blueprints/BASIC_FPSCharacter/FPSWeapons/BaseFPSWeapon/BP_BASIC_WPN_FPS_BaseWeapon` (`self.Get Current Base Weapon`)))
  (`/Game/TPSFPSCharacterSystem/Blueprints/COMMON_ShootingAnimationController/BP_ShootingAnimationController.SetCommonShootAnimPreset` (`self.BP_ShootingAnimController`) (`/Game/TPSFPSCharacterSystem/Blueprints/COMMON_WeaponSystem/BP_WeaponSystem.GetWeaponFireRate` (`self.BP_WeaponSystem`)) (`/Game/TPSFPSCharacterSystem/Blueprints/BASIC_BaseCharacter/Data/BP_BASIC_WPN_BaseWeapon.Get3RDPPShootingAnimProperties` _asbp_basic_wpn_base_weapon) (`/Game/TPSFPSCharacterSystem/Blueprints/BASIC_FPSCharacter/FPSWeapons/BaseFPSWeapon/BP_BASIC_WPN_FPS_BaseWeapon.1st Person Part Shooting Animation Properties` _asbp_basic_wpn_fps_base_weapon)))

(fn `SetCameraMode`
  (params (`Camera Mode` :type "/Game/TPSFPSCharacterSystem/Blueprints/BASIC_FPSCharacter/Data/ENUM_BASIC_FPS_TPS_CAM_MODE Enum" :default "NewEnumerator0"))
  (set `self.Camera Mode` `Camera Mode`))

(fn `SetInChangingCameraMode`
  (params (`In Changing Camera Mode?` :type Boolean))
  (set `self.In Changing Camera Mode?` `In Changing Camera Mode?`))

(fn `UserConstructionScript`
  (`parent.UserConstructionScript`))